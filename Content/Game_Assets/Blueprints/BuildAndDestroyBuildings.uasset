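; An actor that automatically cycles buildings through ghost, construction and destruction by driving the RTS player controller.
; A Tick counter passes three time thresholds, with flags gating each stage, then resets to loop.
; Ghosts spawn from paired building-type and location-actor lists.
; BuildingMaster actors that begin overlapping it are collected and handed to the controller for destruction.
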(event `self.ReceiveBeginPlay`
  (bind _asmy_rtsplayer_controller (cast `MyRTSPlayerController` (`GameplayStatics.GetPlayerController` 0)))
  (set `self.PC` _asmy_rtsplayer_controller))

(event `self.ReceiveActorBeginOverlap`
  (params (OtherActor :type "Actor Object Reference"))
  (bind _asbuilding_master (cast `BuildingMaster` OtherActor))
  (`KismetArrayLibrary.Array_Add` (`self.BuildingList`) _asbuilding_master))

(event `self.ReceiveTick`
  (params (DeltaSeconds :type "Float (single-precision)"))
  (bind _output_get (set `self.Counter` (+ DeltaSeconds (`self.Counter`))))
  (if (> _output_get (`self.BuildingGhostCount`))
    (if (`self.HasGhost`)
      (if (> (`self.Counter`) (`self.BuildingBuildCount`))
        (if (`self.HasBuilt`)
          (if (> (`self.Counter`) (`self.BuildingDestructionCount`))
            (`MyRTSPlayerController.AutoDestroyBuilding` (`self.PC`) (`self.BuildingList`))
            (`KismetArrayLibrary.Array_Clear` (`self.BuildingList`))
            (set `self.HasGhost` false)
            (set `self.HasBuilt` false)
            (set `self.Counter` 0.0))
          (else
            (`MyRTSPlayerController.AutoConstructBuilding` (`self.PC`))
            (set `self.HasBuilt` true))))
      (else
        (for (_array_element _array_index) (`self.LocationList`)
          (`MyRTSPlayerController.AutoGhostBuilding` (`self.PC`) (`|GetArrayItem` (`self.WhatBuildingList`) _array_index) (`self.K2_GetActorLocation` _array_element)))
        (set `self.HasGhost` true)))))

(fn `UserConstructionScript`)