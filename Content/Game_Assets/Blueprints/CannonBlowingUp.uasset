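; Cannon debris actor that shatters its mesh on spawn and removes itself shortly afterwards.
; BeginPlay applies overwhelming damage with a directional impulse at the mesh's location to blow it apart.
; Tick accumulates elapsed time and destroys the actor after about two seconds.
; A timer to set CanLower is longer than that lifetime, so it never fires, and nothing here reads the flag.
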(event `self.ReceiveBeginPlay`
  (bind _mesh (`self.Mesh`))
  (`KismetSystemLibrary.K2_SetTimer` null "LowerFunction" 4.0)
  (`DestructibleComponent.ApplyDamage` _mesh 100000000.0 (`SceneComponent.K2_GetComponentLocation` _mesh) (`self.ImpulseDirection`) 1000.0)
  (set `self.CanLower` false))

(event `self.ReceiveTick`
  (params (DeltaSeconds :type "Float (single-precision)"))
  (bind _output_get (set `self.DeathCountdown` (+ DeltaSeconds (`self.DeathCountdown`))))
  (if (> _output_get 2.0)
    (`self.K2_DestroyActor`)))

(fn `LowerFunction`
  (set `self.CanLower` true))

(fn `UserConstructionScript`)