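; Actor that keeps the RTS camera pawn inside rectangular map bounds.
; On BeginPlay it caches the pawn controlled by MyRTSPlayerController and reads the min and max corners from the TargetLower and TargetHigher actors.
; Every Tick it teleport-free repositions the pawn to clamp X and Y to those corners, leaving Z untouched.
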(event `self.ReceiveBeginPlay`
  (bind _asmy_rtsplayer_controller (cast `MyRTSPlayerController` (`GameplayStatics.GetPlayerController` 0)))
  (set `self.CameraPawn` (`Controller.K2_GetPawn` _asmy_rtsplayer_controller))
  (set `self.StartConstraint` (`self.K2_GetActorLocation` (`self.TargetLower`)))
  (set `self.EndConstraint` (`self.K2_GetActorLocation` (`self.TargetHigher`))))

(event `self.ReceiveTick`
  (params (DeltaSeconds :type "Float (single-precision)"))
  (bind _camerapawn (`self.CameraPawn`))
  (bind (_startconstraint_x _startconstraint_y) (`KismetMathLibrary.BreakVector` (`self.StartConstraint`)))
  (bind _camerapawn_2 (`self.CameraPawn`))
  (bind (_endconstraint_x _endconstraint_y) (`KismetMathLibrary.BreakVector` (`self.EndConstraint`)))
  (bind (_returnvalue_x _returnvalue_y _returnvalue_z) (`KismetMathLibrary.BreakVector` (`self.K2_GetActorLocation` _camerapawn)))
  (bind (_returnvalue_x_2 _returnvalue_y_2 _returnvalue_z_2) (`KismetMathLibrary.BreakVector` (`self.K2_GetActorLocation` _camerapawn_2)))
  (if (< _returnvalue_x_2 _startconstraint_x)
    (`self.K2_SetActorLocation` _camerapawn_2 (`KismetMathLibrary.MakeVector` _startconstraint_x _returnvalue_y_2 _returnvalue_z_2) false false))
  (if (< _returnvalue_y_2 _startconstraint_y)
    (`self.K2_SetActorLocation` _camerapawn_2 (`KismetMathLibrary.MakeVector` _returnvalue_x_2 _startconstraint_y _returnvalue_z_2) false false))
  (if (> _returnvalue_x _endconstraint_x)
    (`self.K2_SetActorLocation` _camerapawn (`KismetMathLibrary.MakeVector` _endconstraint_x _returnvalue_y _returnvalue_z) false false))
  (if (> _returnvalue_y _endconstraint_y)
    (`self.K2_SetActorLocation` _camerapawn (`KismetMathLibrary.MakeVector` _returnvalue_x _endconstraint_y _returnvalue_z) false false)))

(fn `UserConstructionScript`)