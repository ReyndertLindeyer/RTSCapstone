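; An actor for an exploding construction yard that shatters its mesh as soon as play begins.
; BeginPlay applies massive damage with an impulse at the mesh's location and starts a four-second timer.
; The timer's LowerFunction sets CanLower, which Tick checks, but that branch is empty, so no lowering happens.
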(event `self.ReceiveBeginPlay`
  (`KismetSystemLibrary.K2_SetTimer` null "LowerFunction" 4.0)
  (`DestructibleComponent.ApplyDamage` (`self.Mesh`) 100000000.0 (`SceneComponent.K2_GetComponentLocation` (`self.Mesh`)) (`self.ImpulseDirection`) 1000.0)
  (set `self.CanLower` false))

(event `self.ReceiveTick`
  (params (DeltaSeconds :type "Float (single-precision)"))
  (if (`self.CanLower`)
    _))

(fn `LowerFunction`
  (set `self.CanLower` true))

(fn `UserConstructionScript`)