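; UnitCollectionArea is an RTS trigger volume that gathers units and sends them to its waypoint.
; On actor overlap, it adds AvBT, Scout, Rifleman, Rocketeer and MBT units to UnitsFound through separate casts.
; Once a second has elapsed, Tick disables the box collider and passes the list to MyRTSPlayerController's MoveUnitsToLocation.
; The timer never resets, so that move order repeats every frame afterwards.
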(event `self.ReceiveActorBeginOverlap`
  (params (OtherActor :type "Actor Object Reference"))
  (bind _unitsfound (`self.UnitsFound`))
  (bind _asunit_av_bt (cast `UNIT_AvBT` OtherActor)
    (:`then`
      (`KismetArrayLibrary.Array_Add` _unitsfound _asunit_av_bt))
    (:`CastFailed`
      _))
  (bind _asunit_scout (cast `UNIT_Scout` OtherActor)
    (:`then`
      (`KismetArrayLibrary.Array_Add` _unitsfound _asunit_scout))
    (:`CastFailed`
      _))
  (bind _asunit_rifleman (cast `UNIT_Rifleman` OtherActor)
    (:`then`
      (`KismetArrayLibrary.Array_Add` _unitsfound _asunit_rifleman))
    (:`CastFailed`
      _))
  (bind _asunit_rocketeer (cast `UNIT_Rocketeer` OtherActor)
    (:`then`
      (`KismetArrayLibrary.Array_Add` _unitsfound _asunit_rocketeer))
    (:`CastFailed`
      _))
  (bind _asunit_mbt (cast `UNIT_MBT` OtherActor))
  (`KismetArrayLibrary.Array_Add` _unitsfound _asunit_mbt))

(event `self.ReceiveTick`
  (params (DeltaSeconds :type "Float (single-precision)"))
  (bind _output_get (set `self.timer` (+ (`self.timer`) DeltaSeconds)))
  (if (>= _output_get 1.0)
    (`PrimitiveComponent.SetCollisionEnabled` (`self.BoxCollider`) "NoCollision")
    (bind _asmy_rtsplayer_controller (cast `MyRTSPlayerController` (`GameplayStatics.GetPlayerController` 0)))
    (`MyRTSPlayerController.MoveUnitsToLocation` _asmy_rtsplayer_controller (`self.UnitsFound`) (`SceneComponent.K2_GetComponentLocation` (`self.Waypoint`)))))

(fn `UserConstructionScript`)