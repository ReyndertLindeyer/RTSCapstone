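; FlyingPlayerCamera is an actor that drives the RTS player controller's pawn as a flying camera, panning or orbiting around the actor.
; On BeginPlay it moves the pawn to its own location; Tick then pans along PanDirection or, once P or Q enables rotation, advances the orbit.
; RotateAroundPoint derives yaw from the direction to the pawn's previous position, offset 90 degrees, plus a pitch offset.
; Nothing here sets ShouldPan or clears ShouldRotate.
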(event `self.ReceiveBeginPlay`
  (bind _asmy_rtsplayer_controller (cast `MyRTSPlayerController` (`GameplayStatics.GetPlayerController` 0)))
  (bind _output_get (set `self.CameraPawn` (`Controller.K2_GetPawn` _asmy_rtsplayer_controller)))
  (`self.K2_SetActorLocation` _output_get (`self.K2_GetActorLocation`) false false)
  (`self.K2_SetActorRotation` _output_get (struct :`Pitch` -10.0 :`Yaw` 180.0) false))

(event `self.ReceiveTick`
  (params (DeltaSeconds :type "Float (single-precision)"))
  (if (`self.ShouldPan`)
    (`self.K2_AddActorWorldOffset` (`self.CameraPawn`) (* (`self.PanDirection`) 8.0) false false)
    (elif (`self.ShouldRotate`)
      (set `self.CurrentRotation` (+ (`self.CurrentRotation`) (* DeltaSeconds (`self.RotationSpeed`))))
      (`self.RotateAroundPoint`))))

(event `Key|P`
  (params (Key :type "Key Structure"))
  (:`Pressed`
    (set `self.ShouldRotate` true)))

(event `Key|Q`
  (params (Key :type "Key Structure"))
  (:`Pressed`
    (set `self.ShouldRotate` true)))

(fn `RotateAroundPoint`
  (bind _returnvalue (+ (`self.K2_GetActorLocation`) (`KismetMathLibrary.RotateAngleAxis` (`KismetMathLibrary.MakeVector` (`self.RotationRadius`) 0.0 (`self.RotationHeight`)) (* (`self.RotationSpeed`) (`self.CurrentRotation`)) (0.0 0.0 1.0))))
  (`self.K2_SetActorLocationAndRotation` (`self.CameraPawn`) _returnvalue (`KismetMathLibrary.MakeRotator` (.roll (`KismetMathLibrary.FindLookAtRotation` _returnvalue (`self.K2_GetActorLocation` (`self.CameraPawn`)))) (+ (.pitch (`KismetMathLibrary.FindLookAtRotation` _returnvalue (`self.K2_GetActorLocation` (`self.CameraPawn`)))) (`self.RotationAngle`)) (+ (.yaw (`KismetMathLibrary.FindLookAtRotation` _returnvalue (`self.K2_GetActorLocation` (`self.CameraPawn`)))) -90.0)) false false)
  (return))

(fn `UserConstructionScript`)