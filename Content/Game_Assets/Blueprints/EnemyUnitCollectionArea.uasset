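; EnemyUnitCollectionArea is an overlap area that gathers RTS units and directs them to its Waypoint component.
; Entering Grinder, Gattling, Prism and Roomba units are added to UnitsFound, and exiting Characters are removed from it.
; Every Tick, it passes that list and the waypoint's world location to MoveUnitsToLocation on player 0's MyRTSPlayerController, so move orders are reissued each frame through the player's controller.
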(event `self.ReceiveActorBeginOverlap`
  (params (OtherActor :type "Actor Object Reference"))
  (bind _unitsfound (`self.UnitsFound`))
  (bind _asunit_grinder (cast `UNIT_Grinder` OtherActor)
    (:`then`
      (`KismetArrayLibrary.Array_Add` _unitsfound _asunit_grinder))
    (:`CastFailed`
      _))
  (bind _asunit_gattling (cast `UNIT_Gattling` OtherActor)
    (:`then`
      (`KismetArrayLibrary.Array_Add` _unitsfound _asunit_gattling))
    (:`CastFailed`
      _))
  (bind _asunit_prism (cast `UNIT_Prism` OtherActor)
    (:`then`
      (`KismetArrayLibrary.Array_Add` _unitsfound _asunit_prism))
    (:`CastFailed`
      _))
  (bind _asunit_roomba (cast `UNIT_Roomba` OtherActor))
  (`KismetArrayLibrary.Array_Add` _unitsfound _asunit_roomba))

(event `self.ReceiveTick`
  (params (DeltaSeconds :type "Float (single-precision)"))
  (bind _asmy_rtsplayer_controller (cast `MyRTSPlayerController` (`GameplayStatics.GetPlayerController` 0)))
  (`MyRTSPlayerController.MoveUnitsToLocation` _asmy_rtsplayer_controller (`self.UnitsFound`) (`SceneComponent.K2_GetComponentLocation` (`self.Waypoint`))))

(event `self.ReceiveActorEndOverlap`
  (params (OtherActor :type "Actor Object Reference"))
  (bind _unitsfound (`self.UnitsFound`))
  (bind _ascharacter (cast `Character` OtherActor))
  (`KismetArrayLibrary.Array_Remove` _unitsfound (`KismetArrayLibrary.Array_Find` _unitsfound _ascharacter)))

(fn `UserConstructionScript`)